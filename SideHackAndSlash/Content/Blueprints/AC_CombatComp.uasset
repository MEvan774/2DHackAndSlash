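; Combat actor component that drives PaperZD 2D attack combos, hit damage and hurt reactions for its owner.
; Attack events feed normal or up-attack entries from a weapon data asset into ComboCounter2D, which messages the owner and jumps to the Attacking node.
; OnAttack box-traces ahead, records the hit actor and applies damage.
; A montage-based combo variant exists but is never called, and input-buffer logic is disconnected.
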(event `self.ReceiveBeginPlay`
  (bind _returnvalue (`self.GetOwner`))
  (set `self.PaperZDcomp` (`Actor.GetComponentByClass` _returnvalue "/Script/PaperZD.PaperZDAnimationComponent"))
  (set `self.PaperFlipBook\\` (`Actor.GetComponentByClass` _returnvalue "/Script/Paper2D.PaperFlipbookComponent")))

(event `OnSelfDamaged`
  (`PaperZDAnimInstance.JumpToNode` (`PaperZDAnimationComponent.AnimInstance` (`self.PaperZDcomp`)) "Damaged" "None"))

(event `OnAttacking`
  (params (NewParam :type "/Game/Input/Actions/Enum_InputActions Enum" :default "NewEnumerator0"))
  (switch `/Game/Input/Actions/Enum_InputActions` NewParam
    (:`NewEnumerator0`
      (`self.ComboCounter2D` (`/Game/Characters/PDA_Weapon.ComboA` (`self.DAWEP`))))
    (:`NewEnumerator1`
      (`self.ComboCounter2D` (`|MakeArray` (`/Game/Characters/PDA_Weapon.UpAttack` (`self.DAWEP`)))))))

(event `OnAttack`
  (bind _returnvalue (`self.GetOwner`))
  (bind _returnvalue_2 (`Actor.K2_GetActorLocation` _returnvalue))
  (bind _outhit (`KismetSystemLibrary.BoxTraceSingle` :`Start` _returnvalue_2 :`End` (+ _returnvalue_2 (* (`KismetMathLibrary.GetForwardVector` (`Actor.K2_GetActorRotation` _returnvalue)) (90.0 0.0 0.0))) :`HalfSize` (80.0 10.0 45.0) :`TraceChannel` "TraceTypeQuery3" :`DrawDebugType` "ForOneFrame"))
  (bind (_bblockinghit _binitialoverlap _time _distance _location _impactpoint _normal _impactnormal _physmat _hitactor) (`GameplayStatics.BreakHitResult` _outhit))
  (`KismetSystemLibrary.PrintString` (`KismetSystemLibrary.GetDisplayName` _hitactor))
  (`KismetArrayLibrary.Array_AddUnique` (`self.ActorsHit`) _hitactor)
  (`GameplayStatics.ApplyDamage` _hitactor (`KismetMathLibrary.Conv_IntToDouble` (`self.Damage Value`)) null null "/Script/Engine.DamageType"))