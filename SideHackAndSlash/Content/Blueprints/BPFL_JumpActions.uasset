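; Blueprint function library of jump helpers for character movement, covering coyote/multi-jump velocity and variable jump gravity.
; JumpAction checks coyote count or jump count against MaxJumpApexAttemptsPerSimulation, then, when airborne, derives a new Z velocity from current Z velocity and JumpZVelocity.
; GravityRegulator picks a rising, falling or default gravity scale from held input and vertical velocity.
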(fn `GravityRegulator`
  (params (IsHoldingInput :type Boolean) (Velocity :type "Vector Structure") (MoveUpVel :type "Float (double-precision)") (MoveDownVel :type "Float (double-precision)") (DefGravity :type "Float (double-precision)"))
  (returns (GravityOutput :type "Float (double-precision)"))
  (locals (ZVel :type "Float (double-precision)") (GravityScale :type "Float (double-precision)" :default 0.0))
  (set `local.ZVel` (.z Velocity))
  (if (and (== (`local.IsHoldingInput`) true) (> (`local.ZVel`) 0.0))
    (set `local.GravityScale` (`local.MoveUpVel`))
    (return (`local.GravityScale`))
    (elif (or (== (`local.IsHoldingInput`) false) (< (`local.ZVel`) 0.0))
      (set `local.GravityScale` (`local.MoveDownVel`))
      (return (`local.GravityScale`))
      (else
        (if (== (`local.ZVel`) 0.0)
          (set `local.GravityScale` (`local.DefGravity`)))
        (return (`local.GravityScale`))))))

(fn `JumpAction`
  (params (CoyoteCount :type "Float (double-precision)") (CharacterMovement :type "SSTCharacterMovementComponent Object Reference") (JumpAmount :type Integer))
  (returns (VelZ :type "Float (double-precision)"))
  (locals (Gravity :type "Float (double-precision)" :default 0.0) (JumpSpeed :type "Float (double-precision)" :default 0.0))
  (if (or (> CoyoteCount 0.0) (< JumpAmount (`CharacterMovementComponent.MaxJumpApexAttemptsPerSimulation` (`local.CharacterMovement`))))
    (if (not (`NavMovementComponent.IsMovingOnGround` (`local.CharacterMovement`)))
      (set `local.Gravity` (.z (`MovementComponent.Velocity` (`local.CharacterMovement`))))
      (set `local.JumpSpeed` (`KismetMathLibrary.Sqrt` (* (* (`local.Gravity`) -2.0) (`CharacterMovementComponent.JumpZVelocity` (`local.CharacterMovement`)))))
      (if (> (`local.Gravity`) 0.0)
        (set `local.JumpSpeed` (`KismetMathLibrary.FMax` (- (`local.JumpSpeed`) (`local.Gravity`))))
        (elif (< (`local.Gravity`) 0.0)
          _
          (else
            _)))
      (return (+ (`local.Gravity`) (`local.JumpSpeed`))))))